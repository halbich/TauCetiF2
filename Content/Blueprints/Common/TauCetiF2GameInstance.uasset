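; TauCetiF2GameInstance holds level-loading state and the current error for the game.
; LoadGame, StartNewGame and LoadMainMenu reset progress with a Czech loading message and set the load method and save path.
; The first two open the LoadingScreen level, with StartNewGame also storing a new-game carrier, while LoadMainMenu opens MainMenu directly.
; SetLoadState updates percent and message, while SetError flags any non-empty message for GetError to return.
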(fn `Get Error`
  (returns (`Has Error` :type Boolean) (`Error Text` :type String))
  (return (`self.Has Error`) (`self.Error Message`)))

(fn `Load Game`
  (params (`Level To Load` :type String))
  (set `self.Current Load Message` "Nahrávám hru")
  (set `self.Loaded Percent` 0)
  (set `self.Load Game Path` `Level To Load`)
  (set `self.Load Level Method` "NewEnumerator2")
  (`GameplayStatics.OpenLevel` "LoadingScreen"))

(fn `Load Main Menu`
  (params (`Level To Load` :type String))
  (set `self.Current Load Message` "Nahrávám hru")
  (set `self.Loaded Percent` 0)
  (set `self.Load Game Path` "")
  (set `self.Load Level Method` "NewEnumerator0")
  (`GameplayStatics.OpenLevel` "MainMenu"))

(fn `Set Error`
  (params (Message :type String))
  (set `self.Has Error` (> (`KismetStringLibrary.Len` Message) 0))
  (set `self.Error Message` Message))

(fn `SetLoadState`
  (params (Percent :type Integer) (Message :type Text))
  (set `self.Current Load Message` Message)
  (set `self.Loaded Percent` Percent))

(fn `Start New Game`
  (params (`Level To Load` :type "SaveGameCarrier Object Reference"))
  (set `self.Current Load Message` "Nahrávám hru")
  (set `self.Loaded Percent` 0)
  (set `self.Load Game Path` "")
  (set `self.Load Level Method` "NewEnumerator1")
  (set `self.New Game Carrier` `Level To Load`)
  (`GameplayStatics.OpenLevel` "LoadingScreen"))