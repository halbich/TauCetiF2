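; Ambient music player actor that plays random songs from either a main-menu or in-game sound bank, chosen when StartPlaying is called.
; Each song is set on a single audio component and announced through a newly created song info widget.
; When a song finishes, it waits a random delay from the active bank, then plays another, re-waiting while music or master volume is zero.
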(event `self.AudioComponent.OnAudioFinished`
  (bind (_mindelay _maxdelay _usingdefinitions) (break `/Game/Blueprints/Common/SoundSourceDefinition` (select `bool` (`self.IsMainMenu`) :`false` (`self.InGameSource`) :`true` (`self.MenuSource`))))
  (`KismetSystemLibrary.Delay` (`KismetMathLibrary.RandomFloatInRange` _mindelay _maxdelay) :!label _label)
  (bind _resultvalue (`Helpers.GetSoundClassVolume` "/Game/Sounds/TCF2Music.TCF2Music"))
  (bind _resultvalue_2 (`Helpers.GetSoundClassVolume` "/Game/Sounds/TCF2Master.TCF2Master"))
  (if (> (* _resultvalue_2 _resultvalue) 0.0)
    (`self.PlaySound` (`self.RandomSound` _usingdefinitions))
    (else
      (goto _label))))

(fn `PlayRandomSoundFromBank`
  (`self.PlaySound` (`self.RandomSound` (`.UsingDefinitions_13_19A4C3B74D41B8C0E1D5C4957C93F677` (break `/Game/Blueprints/Common/SoundSourceDefinition` (select `bool` (`self.IsMainMenu`) :`false` (`self.InGameSource`) :`true` (`self.MenuSource`)))))))

(fn `PlaySound`
  (params (Source :type "/Game/Blueprints/Common/SoundSourceDefinitionItem Structure"))
  (bind (_sound _displaytext) (break `/Game/Blueprints/Common/SoundSourceDefinitionItem` Source))
  (bind _audiocomponent (`self.AudioComponent`))
  (bind _returnvalue (`|CreateWidget` "/Game/UMG/Widgets/SongInfoWidget.SongInfoWidget_C"))
  (`/Game/UMG/Widgets/SongInfoWidget.ShowSongInfo` _returnvalue _displaytext)
  (`AudioComponent.SetSound` _audiocomponent _sound)
  (`AudioComponent.Play` _audiocomponent 0.0))

(fn `StartPlaying`
  (params (IsMainMenu :type Boolean))
  (set `self.IsMainMenu` IsMainMenu)
  (`self.PlayRandomSoundFromBank`))

(fn `UserConstructionScript`)