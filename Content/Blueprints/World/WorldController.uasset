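; World controller actor that saves and loads the world's blocks and offers debug keys.
; Save To Carrier writes UsedBlocks into the passed save game object, and Load From Carrier feeds them back through LoadBlocksArray, with a noted engine-error workaround.
; BeginPlay flags loading as done after a zero-length delay.
; H toggles between drawing min/max debug boxes and flushing debug lines, while J prints a test message.
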(event EventBeginPlay
  (Utilities|FlowControl|Delay 0.0)
  (Variables|Default|SetIsLoadingDone true))

(event EventActorBeginOverlap
  (params (OtherActor :type Actor%20Object%20Reference)))

(event EventTick
  (params (DeltaSeconds :type Float%20%28single-precision%29)))

(event Input|KeyboardEvents|H
  (params (Key :type Key%20Structure :default "AnyKey"))
  (:Pressed
    (Utilities|FlowControl|FlipFlop
      (:A
        (Class|WorldController|DEBUGShowMinMaxBoxes))
      (:B
        (Rendering|Debug|FlushPersistentDebugLines)))))

(event Input|KeyboardEvents|J
  (params (Key :type Key%20Structure :default "AnyKey"))
  (:Pressed
    (Development|PrintString "Hello")))

(fn ConstructionScript)

(fn LoadfromCarrier
  (params (Save%20Game :type Save%20Game%20Carrier%20Object%20Reference))
  ;[1 1 1] Workaround engine error
  (bind _output_get (LocalVariables|Setblocks (Variables|/Script/TauCetiF2.SaveGameCarrier|GetUsedBlocks Save%20Game)))
  (Class|WorldController|LoadBlocksArray _output_get))

(fn SavetoCarrier
  (params (Save%20Game :type Save%20Game%20Carrier%20Object%20Reference))
  (LocalVariables|Setsave Save%20Game)
  (Variables|/Script/TauCetiF2.SaveGameCarrier|SetUsedBlocks (LocalVariables|Getsave) (Variables|Default|GetUsedBlocks))
  (return (LocalVariables|Getsave)))