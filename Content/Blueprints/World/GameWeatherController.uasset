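; GameWeatherController is an actor that animates cloud speed on the level's Sky_BP, found at BeginPlay.
; Each Tick moves a time value back and forth along a float curve, reversing direction at the curve's maximum time and at zero.
; The sampled value becomes the sky's cloud speed and is pushed into its material parameter, while cloud opacity is held at full.
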(event `self.ReceiveBeginPlay`
  (bind _outactors (`GameplayStatics.GetAllActorsOfClass` "/Game/Blueprints/World/Sky_BP.Sky_BP_C"))
  (set `self.SkyBP` (`KismetArrayLibrary.Array_Get` _outactors)))

(event `self.ReceiveTick`
  (params (DeltaSeconds :type "Float (single-precision)"))
  (bind _skybp (`self.SkyBP`))
  (bind (_mintime _maxtime) (`CurveBase.GetTimeRange` (`self.curve`)))
  (bind _returnvalue (+ (* DeltaSeconds (`self.CurrentSpeed`)) (`self.ActualTime`)))
  (if (>= _returnvalue _maxtime)
    (set `self.CurrentSpeed` -1.0)
    (elif (<= _returnvalue 0.0)
      (set `self.CurrentSpeed` 1.0)))
  (bind _output_get (set `self.ActualTime` (`KismetMathLibrary.FClamp` _returnvalue _mintime _maxtime)))
  (bind _output_get_2 (set `self.CurrentCloudSpeed` (`CurveFloat.GetFloatValue` (`self.curve`) _output_get)))
  (bind _output_get_3 (set `/Game/Blueprints/Engine/BP_Sky_SphereWithLightComponent.Cloud speed` _output_get_2 _skybp))
  (set `/Game/Blueprints/Engine/BP_Sky_SphereWithLightComponent.Cloud opacity` 1.0 _skybp)
  (`MaterialInstanceDynamic.SetScalarParameterValue` (`/Game/Blueprints/Engine/BP_Sky_SphereWithLightComponent.Sky material` _skybp) "Cloud speed" _output_get_3))

(fn `UserConstructionScript`)