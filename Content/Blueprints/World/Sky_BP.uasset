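; Sky actor that runs a looping day/night cycle on a parent sky Blueprint's sun direction logic.
; Tick advances a wrapped time, scaled from day length, that drives the directional light's pitch through a curve.
; Sun height then sets sun and skylight intensities via curves and fires a notification when night state flips.
; Construction sets the starting part of day and can preview it in the editor.
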(event `self.ReceiveTick`
  (params (DeltaSeconds :type "Float (single-precision)"))
  (set `self.CurrentTime` (mod (+ (* DeltaSeconds (`self.DayMultiplier`)) (`self.CurrentTime`)) (`self.MaxTime`)))
  (`self.UpdateLight`))

(fn `CheckNight`
  (params (`Sun Height` :type "Float (double-precision)"))
  (bind _output_get (set `self.IsNight` (<= `Sun Height` (`self.SunDayHeightValue`))))
  (if (!= _output_get (`self.IsNightPrevious`))
    (bind _output_get_2 (set `self.IsNightPrevious` _output_get))
    (`self.On Night Changed` _output_get_2))
  (return))

(fn `Update Intensities`
  (returns (`Sun height` :type "Float (double-precision)"))
  (bind _sun_height (`self.Sun height`))
  (`LightComponent.SetIntensity` (`self.LIght Source`) (`CurveFloat.GetFloatValue` (`self.LightIntensityCurve`) _sun_height))
  (`SkyLightComponent.SetIntensity` (`self.SkyLight`) (`CurveFloat.GetFloatValue` (`self.SkyLightCurve`) _sun_height))
  (return _sun_height))

(fn `UpdateLight`
  (`SceneComponent.K2_SetRelativeLocationAndRotation` (`self.LIght Source`) (0.0 0.0 0.0) (`KismetMathLibrary.MakeRotator` 0.0 (.y (`CurveVector.GetVectorValue` (`self.LightSourceCurve`) (`self.CurrentTime`)))) false false)
  (`self.UpdateSunDirection`)
  (bind _sun_height (`self.Update Intensities`))
  (`self.CheckNight` _sun_height)
  (return))

(fn `UserConstructionScript`
  (`parent.UserConstructionScript`)
  (set `self.Directional light component` (`self.LIght Source`))
  (bind _output_get (set `self.MaxTime` (`.MaxTime` (`CurveBase.GetTimeRange` (`self.LightSourceCurve`)))))
  (set `self.DayMultiplier` (/ _output_get (`self.DayLength`)))
  (set `self.CurrentTime` (* _output_get (`self.PartOfDay`)))
  (if (`self.UpdatePartOfDayInEditor`)
    (`self.UpdateLight`)))